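; BP_DinoGamestate is the game state for Dino's Revenge and holds the level's victory check.
; CheckVictoryCondition searches the world for Tesla guns, AI soldiers, the bunker and the AI boss.
; When none of them remain, it casts the first player pawn to BP_Dino and calls VictoryMessage on it.
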(event Custom|CheckVictoryCondition
  (bind _outactors (Actor|GetAllActorsOfClass "/Game/DinosRevengeContent/Meshes/TeslaGun/BP_TeslaGun.BP_TeslaGun_C"))
  (bind _outactors_2 (Actor|GetAllActorsOfClass "/Game/DinosRevengeContent/Characters/Humans/BP_AISoldier.BP_AISoldier_C"))
  (bind _returnvalue (Actor|GetActorOfClass "/Game/DinosRevengeContent/Meshes/MilitaryBunker/BP_Bunker.BP_Bunker_C"))
  (bind _returnvalue_2 (Actor|GetActorOfClass "/Game/DinosRevengeContent/Characters/Humans/Boss/BP_AIBoss.BP_AIBoss_C"))
  (if (Math|Boolean|ANDBoolean (not (Utilities|IsValid _returnvalue_2)) (not (Utilities|IsValid _returnvalue)) (== (+ (Utilities|Array|Length _outactors_2) (Utilities|Array|Length _outactors)) 0))
    (bind _asbp_dino (Utilities|Casting|CastToBP_Dino (Game|Player|GetPlayerPawn 0)))
    (Default|VictoryMessage _asbp_dino)))

(fn ConstructionScript)