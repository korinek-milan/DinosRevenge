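; Military bunker actor that spawns AI soldiers and can be destroyed.
; A dino entering the trigger starts, once and after a delay, a looping timer that spawns soldiers with the bunker's move points and a randomized start flag.
; Soldiers entering or leaving the box toggle timeline-driven sliding doors.
; Each Kill/Destroy call lowers health, adding fires at set thresholds, then exploding and destroying the actor at zero.
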(event OnComponentBeginOverlap(Box)
  (params (OverlappedComponent :type Primitive%20Component%20Object%20Reference) (OtherActor :type Actor%20Object%20Reference) (OtherComp :type Primitive%20Component%20Object%20Reference) (OtherBodyIndex :type Integer) (bFromSweep :type Boolean) (SweepResult :type Hit%20Result%20Structure%20%28by%20ref%29))
  (Utilities|Casting|CastToBP_AISoldier OtherActor)
  (CallFunction|OpenCloseDoor))

(event OnComponentEndOverlap(Box)
  (params (OverlappedComponent :type Primitive%20Component%20Object%20Reference) (OtherActor :type Actor%20Object%20Reference) (OtherComp :type Primitive%20Component%20Object%20Reference) (OtherBodyIndex :type Integer))
  (Utilities|Casting|CastToBP_AISoldier OtherActor)
  (CallFunction|OpenCloseDoor))

(event OnComponentBeginOverlap(StartSpawning)
  (params (OverlappedComponent :type Primitive%20Component%20Object%20Reference) (OtherActor :type Actor%20Object%20Reference) (OtherComp :type Primitive%20Component%20Object%20Reference) (OtherBodyIndex :type Integer) (bFromSweep :type Boolean) (SweepResult :type Hit%20Result%20Structure%20%28by%20ref%29))
  (Utilities|Casting|CastToBP_Dino OtherActor)
  (Variables|/Script/Engine.PrimitiveComponent|SetbGenerateOverlapEvents (Variables|Default|GetStartSpawning) false)
  (Utilities|FlowControl|Delay 1e+01)
  (Utilities|Time|SetTimerbyFunctionName 0 "SpawnSoldier" 15.0 true))

(event Custom|OpenCloseDoor
  (if (< (.x (Variables|/Script/Engine.SceneComponent|GetRelativeLocation (Variables|Default|GetLeft))) 0.0)
    (bind _newtrack_0 (Timeline|Timeline_0 Reverse)
      (:Update
        (Transformation|SetRelativeLocation (Variables|Default|GetLeft) (Math|Vector|MakeVector (* _newtrack_0 -1.0) 0.0 0.0) false false)
        (Transformation|SetRelativeLocation (Variables|Default|GetRight) (Math|Vector|MakeVector _newtrack_0 0.0 0.0) false false)))
    (else
      (Timeline|Timeline_0 Play))))

(event Custom|SpawnSoldier
  (bind _returnvalue (AI|SpawnAIFromClass "/Game/DinosRevengeContent/Characters/Humans/BP_AISoldier.BP_AISoldier_C" 0 (Transformation|GetWorldLocation (Variables|Default|GetSpawner)) "0, 0, 0" false 0))
  (bind _asbp_aisoldier (Utilities|Casting|CastToBP_AISoldier _returnvalue))
  (Variables|/Game/DinosRevengeContent/Characters/Humans/BP_AISoldier.BP_AISoldier_C|SetMovePoints _asbp_aisoldier (Variables|Default|GetMovePoints))
  (Default|SetStartValues _asbp_aisoldier (> (Math|Random|RandomIntegerinRange 0 100) 75)))

(event EventKill/Destroy
  (params (HitImpulse :type Vector :default "0, 0, 0"))
  (bind _building (Variables|Default|GetBuilding))
  (bind _engine (Variables|Default|GetEngine))
  (bind _engine_2 (Variables|Default|GetEngine))
  (bind _returnvalue (Transformation|GetWorldLocation _building))
  (bind _output_get (Variables|Default|SetHealth (- (Variables|Default|GetHealth) 1)))
  (switch int _output_get
    (:0
      (Effects|SpawnEmitterAttached "/Game/DinosRevengeContent/Particles/P_Explosion.P_Explosion" _engine "None" (Transformation|GetWorldLocation _engine) "0, 0, 0" "2.000000,2.000000,2.000000" "KeepWorldPosition")
      (Utilities|FlowControl|Delay 0.4)
      (Actor|DestroyActor))
    (:1
      (Effects|SpawnEmitterAttached "/Game/DinosRevengeContent/Particles/P_Fire.P_Fire" _building "None" (Math|Vector|MakeVector (.x _returnvalue) (.y _returnvalue) (+ (.z _returnvalue) 2e+02)) "0, 0, 0" "4.000000,4.000000,4.000000" "KeepWorldPosition"))
    (:3
      (Effects|SpawnEmitterAttached "/Game/DinosRevengeContent/Particles/P_Fire.P_Fire" _engine_2 "None" (Transformation|GetWorldLocation _engine_2) "0, 0, 0" "2.000000,2.000000,2.000000" "KeepWorldPosition"))))

(fn ConstructionScript)