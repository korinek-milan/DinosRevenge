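; Tesla gun turret that tracks the player inside its trigger box and fires a damaging laser beam.
; Tick eases body yaw and sets pitch with a lower limit; a sphere trace on the player starts a charge shown by rising point light intensity.
; At full charge it stops tracking, fires the beam with timed hit checks against BP_Dino, then reloads.
; Each Kill/Destroy call removes health, spawning fire at one left and exploding at zero.
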(event OnComponentBeginOverlap(Box)
  (params (OverlappedComponent :type Primitive%20Component%20Object%20Reference) (OtherActor :type Actor%20Object%20Reference) (OtherComp :type Primitive%20Component%20Object%20Reference) (OtherBodyIndex :type Integer) (bFromSweep :type Boolean) (SweepResult :type Hit%20Result%20Structure%20%28by%20ref%29))
  (if (== OtherActor (Game|Player|GetPlayerPawn 0))
    (Actor|Tick|SetActorTickEnabled true)))

(event OnComponentEndOverlap(Box)
  (params (OverlappedComponent :type Primitive%20Component%20Object%20Reference) (OtherActor :type Actor%20Object%20Reference) (OtherComp :type Primitive%20Component%20Object%20Reference) (OtherBodyIndex :type Integer))
  (if (== OtherActor (Game|Player|GetPlayerPawn 0))
    (Actor|Tick|SetActorTickEnabled false)))

(event Custom|LaserFire
  (bind _gun (Variables|Default|GetGun))
  (bind _particlesystem (Variables|Default|GetParticleSystem))
  (Actor|Tick|SetActorTickEnabled false)
  (Components|Activation|Activate _particlesystem true)
  (Rendering|SetVisibility _particlesystem true false)
  (Class|ParticleSystemComponent|SetBeamSourcePoint _particlesystem 0 (Transformation|GetWorldLocation (Variables|Default|GetLaserStart)))
  (Class|ParticleSystemComponent|SetBeamEndPoint _particlesystem 0 (+ (Transformation|GetWorldLocation _gun) (* (Math|Vector|GetForwardVector _gun) 1e+04)))
  (bind _returnvalue (Utilities|Time|SetTimerbyFunctionName 0 "LaserHitCheck" 0.1 true))
  (Variables|Default|SetLaserTimer _returnvalue)
  (Utilities|FlowControl|Delay 2.0)
  (Rendering|SetVisibility _particlesystem false false)
  (Components|Activation|Deactivate _particlesystem)
  (Utilities|Time|ClearandInvalidateTimerbyHandle (Variables|Default|GetLaserTimer))
  (Actor|Tick|SetActorTickEnabled true)
  (Rendering|Components|Light|SetIntensity (Variables|Default|GetPointLight) 0.0)
  (Utilities|FlowControl|Delay (Variables|Default|GetReloadDuration))
  (CallFunction|FireReady))

(event Custom|LoadFire
  (bind _pointlight (Variables|Default|GetPointLight))
  (bind _intensity (Variables|/Script/Engine.LightComponentBase|GetIntensity _pointlight))
  (Utilities|FlowControl|Gate false :!label _label
    (:Exit
      (if (<= _intensity 1.5e+04)
        (Rendering|Components|Light|SetIntensity _pointlight (+ _intensity 1e+02))
        (else
          (Utilities|FlowControl|DoOnce false
            (:Completed
              (CallFunction|LaserFire)
              (goto _label Close))))))))

(event Custom|EnableGun
  (Variables|/Script/Engine.PrimitiveComponent|SetbGenerateOverlapEvents (Variables|Default|GetBox) true))

(event Custom|FireReady
  (bind _pointlight (Variables|Default|GetPointLight))
  (bind _intensity (Variables|/Script/Engine.LightComponentBase|GetIntensity _pointlight))
  (Utilities|FlowControl|Sequence
    (:then_0
      (Utilities|FlowControl|DoOnce false) ; enters at Reset
    )
    (:then_1
      (Utilities|FlowControl|Gate false) ; enters at Open
    )))

(event Custom|LaserHitCheck
  (bind (_bhit _hitactor) (CallFunction|TraceLaserCollision))
  (if _bhit
    (bind _asbp_dino (Utilities|Casting|CastToBP_Dino _hitactor))
    (Default|GetDamage _asbp_dino (Math|Conversions|ToFloat(Integer) (Variables|Default|GetDamage)))))

(event EventKill/Destroy
  (params (HitImpulse :type Vector :default "0, 0, 0"))
  (bind _output_get (Variables|Default|SetHealth (- (Variables|Default|GetHealth) 1)))
  (switch int _output_get
    (:0
      (Effects|SpawnEmitterAttached "/Game/DinosRevengeContent/Particles/P_Explosion.P_Explosion" (Variables|Default|GetBase) "None" (Transformation|GetWorldLocation (Variables|Default|GetBodyRotator)) "0, 0, 0" "2.000000,2.000000,2.000000" "KeepWorldPosition")
      (Utilities|FlowControl|Delay 0.4)
      (Actor|DestroyActor))
    (:1
      (bind _returnvalue (Effects|SpawnEmitterAttached "/Game/DinosRevengeContent/Particles/P_Fire.P_Fire" (Variables|Default|GetBase) "None" (Transformation|GetWorldLocation (Variables|Default|GetBodyRotator)) "0, 0, 0" "2.000000,2.000000,2.000000" "KeepWorldPosition"))
      (Variables|Default|SetFireEmitter _returnvalue))))

(event EventTick
  (params (DeltaSeconds :type Float%20%28single-precision%29))
  (bind _bodyrotator (Variables|Default|GetBodyRotator))
  (Transformation|SetRelativeRotation _bodyrotator (Math|Rotator|MakeRotator 0.0 0.0 (.yaw (Math|Rotator|Lerp(Rotator) (Variables|/Script/Engine.SceneComponent|GetRelativeRotation _bodyrotator) (Math|Rotator|FindLookatRotation (Transformation|GetWorldLocation _bodyrotator) (Transformation|GetActorLocation (Game|Player|GetPlayerPawn 0))) DeltaSeconds true))) false false)
  (Transformation|SetRelativeRotation (Variables|Default|GetGunRotator) (Math|Rotator|MakeRotator 0.0 (Math|Float|Max(Float) (.pitch (Math|Rotator|FindLookatRotation (Transformation|GetWorldLocation (Variables|Default|GetGunRotator)) (Transformation|GetActorLocation (Game|Player|GetPlayerPawn 0)))) -3e+01) 0.0) false false)
  (if (== (Variables|/Script/Engine.LightComponentBase|GetIntensity (Variables|Default|GetPointLight)) 0.0)
    (bind _bhit (CallFunction|TraceLaserCollision))
    (if _bhit
      (CallFunction|LoadFire))
    (else
      (CallFunction|LoadFire))))

(fn ConstructionScript
  (Variables|/Script/Engine.PrimitiveComponent|SetbGenerateOverlapEvents (Variables|Default|GetBox) (Variables|Default|GetbEnable)))

(fn TraceLaserCollision
  (bind _gun (Variables|Default|GetGun))
  (bind _outhit (Collision|SphereTraceByChannel (Transformation|GetWorldLocation (Variables|Default|GetLaserStart)) (+ (Transformation|GetWorldLocation _gun) (* (Math|Vector|GetForwardVector _gun) 1e+04)) 25.0 "TraceTypeQuery1" false 0 "None"))
  (return (== (.HitActor (Collision|BreakHitResult _outhit)) (Game|Player|GetPlayerPawn 0)) (.HitActor (Collision|BreakHitResult _outhit))))