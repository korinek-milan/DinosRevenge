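; BP_MeshSpline is a spline-based placement Blueprint in the Fence mesh folder that repeats a static mesh along a path.
; Its construction script divides the rounded spline length by SpaceBetween and adds a mesh component at each interval in local space.
; Every copy shares one configurable rotation rather than following the spline's direction.
; The IgnorePlayerCollision flag sets whether the copies ignore or block the Pawn channel.
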(fn ConstructionScript
  (for _index (range 0 (/ (Math|Float|Round (Spline|GetSplineLength (Variables|Default|GetSpline))) (Variables|Default|GetSpaceBetween)))
    (bind _returnvalue (AddComponent|AddStaticMeshComponent false (Math|Transform|MakeTransform (Spline|GetLocationatDistanceAlongSpline (Variables|Default|GetSpline) (Math|Conversions|ToFloat(Integer) (* _index (Variables|Default|GetSpaceBetween))) "Local") (Variables|Default|GetRelative%20Transform%20Rotation) "1.000000,1.000000,1.000000")))
    (Components|StaticMesh|SetStaticMesh _returnvalue (Variables|Default|GetMesh))
    (Collision|SetCollisionResponsetoChannel _returnvalue "ECC_Pawn" (select (Variables|Default|GetbIgnorePlayerCollision) "ECR_Ignore" "ECR_Block"))))