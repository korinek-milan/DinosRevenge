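; Triceratops character Blueprint with a timed charge as its primary attack.
; Pressing the attack locks player move input, sets the Charge flag and raises walk speed.
; A fast looping timer forces movement along the control rotation's yaw, so the charge follows where the controller faces.
; After a few seconds the flag clears, speed drops, input returns and the timer stops.
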(event Custom|Charge
  (Pawn|Input|AddMovementInput (Math|Vector|GetForwardVector (Math|Rotator|MakeRotator 0.0 0.0 (.yaw (Pawn|GetControlRotation :!class /Script/Engine.Pawn)))) 1.0 true))

(event Input|ActionEvents|InputActionPrimaryAttack
  (params (Key :type Key%20Structure :default "None"))
  (bind _returnvalue (Pawn|GetController))
  (:Pressed
    (Input|SetIgnoreMoveInput _returnvalue true)
    (Variables|Default|SetbCharge true)
    (Variables|/Script/Engine.CharacterMovementComponent|SetMaxWalkSpeed (Variables|Character|GetCharacterMovement) 5e+02)
    (bind _returnvalue_2 (Utilities|Time|SetTimerbyFunctionName 0 "Charge" 0.01 true))
    (Variables|Default|SetChargeTimer _returnvalue_2)
    (Utilities|FlowControl|Delay 5.0)
    (Variables|Default|SetbCharge false)
    (Variables|/Script/Engine.CharacterMovementComponent|SetMaxWalkSpeed (Variables|Character|GetCharacterMovement) 1e+02)
    (Input|ResetIgnoreMoveInput _returnvalue)
    (Utilities|Time|ClearandInvalidateTimerbyHandle (Variables|Default|GetChargeTimer))))

(fn ConstructionScript)