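; BP_AIBoss is the human boss character, which plays a little-girl scream at its location on BeginPlay.
; When eaten, it spawns an enlarged blood effect, destroys itself and asks BP_DinoGamestate to check the victory condition.
; When killed by a hit, it drops capsule collision, ragdolls with the impulse as mesh velocity, then after a short delay follows the same path as being eaten.
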(event Custom|Eaten
  (Effects|SpawnEmitteratLocation "/Game/DinosRevengeContent/Particles/Blood/P_Blood.P_Blood" (Transformation|GetWorldLocation (Variables|Character|GetMesh)) "0, 0, 0" "2.000000,2.000000,2.000000")
  (Actor|DestroyActor)
  (bind _asbp_dino_gamestate (Utilities|Casting|CastToBP_DinoGamestate (Game|GetGameState)))
  (Default|CheckVictoryCondition _asbp_dino_gamestate))

(event EventBeginPlay
  (Audio|PlaySoundatLocation "/Game/DinosRevengeContent/Sounds/little-girl-screaming.little-girl-screaming" (Transformation|GetActorLocation) "0, 0, 0" 1.0 1.0 0.0 0 0 0 0))

(event EventKill/Destroy
  (params (HitImpulse :type Vector :default "0, 0, 0"))
  (bind _mesh (Variables|Character|GetMesh))
  (Collision|SetCollisionEnabled (Variables|Collision|GetCapsuleComponent) "NoCollision")
  (Physics|SetSimulatePhysics _mesh true)
  (Physics|SetPhysicsLinearVelocity _mesh HitImpulse false "None")
  (Utilities|FlowControl|Delay 3.0)
  (Effects|SpawnEmitteratLocation "/Game/DinosRevengeContent/Particles/Blood/P_Blood.P_Blood" (Transformation|GetWorldLocation (Variables|Character|GetMesh)) "0, 0, 0" "2.000000,2.000000,2.000000")
  (Actor|DestroyActor)
  (bind _asbp_dino_gamestate (Utilities|Casting|CastToBP_DinoGamestate (Game|GetGameState)))
  (Default|CheckVictoryCondition _asbp_dino_gamestate))

(fn ConstructionScript)