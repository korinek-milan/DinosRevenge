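; AI enemy soldier, in normal or faster-firing Heavy variant, that moves to a random move point and shoots at the player dinosaur on entering its trigger box.
; Looping timers aim body and weapon and fire randomly spread line traces, with a reload pause after MaxBullets.
; Death by ragdoll impulse, falling while engaged, or being eaten spawns blood, destroys the actor and makes the game state check victory.
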(event OnComponentBeginOverlap(Box)
  (params (OverlappedComponent :type Primitive%20Component%20Object%20Reference) (OtherActor :type Actor%20Object%20Reference) (OtherComp :type Primitive%20Component%20Object%20Reference) (OtherBodyIndex :type Integer) (bFromSweep :type Boolean) (SweepResult :type Hit%20Result%20Structure%20%28by%20ref%29))
  (if (== OtherActor (Game|Player|GetPlayerPawn 0))
    (Components|Movement|StopMovementImmediately (Variables|Character|GetCharacterMovement))
    (CallFunction|StartShooting)))

(event OnComponentEndOverlap(Box)
  (params (OverlappedComponent :type Primitive%20Component%20Object%20Reference) (OtherActor :type Actor%20Object%20Reference) (OtherComp :type Primitive%20Component%20Object%20Reference) (OtherBodyIndex :type Integer))
  (if (== OtherActor (Game|Player|GetPlayerPawn 0))
    (CallFunction|StopShooting)))

(event Custom|MoveToPlace
  (bind _movepoints (Variables|Default|GetMovePoints))
  (if (not (Utilities|Array|IsEmpty (Variables|Default|GetMovePoints)))
    (AI|AIMoveTo self (Transformation|GetActorLocation (Utilities|Array|Get(acopy) _movepoints (Math|Random|RandomIntegerinRange 0 (- (Utilities|Array|Length _movepoints) 1)))) 0 5.0 false
      (:OnSuccess
        (Variables|/Script/Engine.PrimitiveComponent|SetbGenerateOverlapEvents (Variables|Default|GetBox) true)))
    (else
      (Variables|/Script/Engine.PrimitiveComponent|SetbGenerateOverlapEvents (Variables|Default|GetBox) true))))

(event Custom|StartShooting
  (bind _returnvalue (Utilities|Time|SetTimerbyFunctionName 0 "RotateTick" 0.1 true))
  (Variables|Default|SetRotateTimer _returnvalue)
  (bind _returnvalue_2 (Utilities|Time|SetTimerbyFunctionName 0 "Shooting" (Variables|Default|GetShootingTime) true))
  (Variables|Default|SetShootingTimer _returnvalue_2))

(event Custom|RotateTick
  (bind _returnvalue (Transformation|GetActorRotation))
  (bind _returnvalue_2 (Transformation|GetActorLocation))
  (bind _returnvalue_3 (Game|Player|GetPlayerPawn 0))
  (bind _weapon (Variables|Default|GetWeapon))
  (bind _returnvalue_4 (Transformation|GetActorLocation _returnvalue_3))
  (bind _relativerotation (Variables|/Script/Engine.SceneComponent|GetRelativeRotation _weapon))
  (bind _returnvalue_5 (Math|Rotator|FindLookatRotation _returnvalue_2 _returnvalue_4))
  (Transformation|SetActorRotation (Math|Rotator|MakeRotator (.roll _returnvalue) (.pitch _returnvalue) (.yaw _returnvalue_5)))
  (Transformation|SetRelativeRotation _weapon (Math|Rotator|MakeRotator (.roll _relativerotation) (* (.pitch _returnvalue_5) -1.0) (.yaw _relativerotation)) false false)
  ;[1 1 1] Falling
  (if (AI|Components|NavMovement|IsFalling (Variables|Character|GetCharacterMovement))
    (bind _output_get (Variables|Default|SetFallTime (+ (Variables|Default|GetFallTime) (Utilities|Time|GetWorldDeltaSeconds))))
    (if (> _output_get 0.1)
      (CallFunction|Kill/Destroy "0, 0, 0"))
    (else
      (Variables|Default|SetFallTime 0.0))))

(event Custom|StopShooting
  (Utilities|Time|ClearandInvalidateTimerbyHandle (Variables|Default|GetRotateTimer))
  (Utilities|Time|ClearandInvalidateTimerbyHandle (Variables|Default|GetShootingTimer)))

(event Custom|Eaten
  (Effects|SpawnEmitteratLocation "/Game/DinosRevengeContent/Particles/Blood/P_Blood.P_Blood" (Transformation|GetWorldLocation (Variables|Character|GetMesh)) "0, 0, 0" "2.000000,2.000000,2.000000")
  (Actor|DestroyActor)
  (bind _asbp_dino_gamestate (Utilities|Casting|CastToBP_DinoGamestate (Game|GetGameState)))
  (Default|CheckVictoryCondition _asbp_dino_gamestate))

(event Custom|Shooting
  (Utilities|FlowControl|Gate false :!label _label
    (:Exit
      (bind _wallhit (CallFunction|TraceandTryHit))
      (if (not _wallhit)
        (Audio|PlaySoundatLocation "/Game/DinosRevengeContent/Sounds/gun_firing_Cue.gun_firing_Cue" (Transformation|GetWorldLocation (Variables|Default|GetWeapon)) "0, 0, 0" 1.0 1.0 0.0 0 0 0 0)
        (bind _output_get (Variables|Default|SetBulletsFired (+ (Variables|Default|GetBulletsFired) 1)))
        (if (>= _output_get (Variables|Default|GetMaxBullets))
          (Utilities|FlowControl|Sequence
            (:then_0
              (goto _label Close))
            (:then_1
              (Audio|PlaySoundatLocation "/Game/DinosRevengeContent/Sounds/rifle-reload_Cue.rifle-reload_Cue" (Transformation|GetWorldLocation (Variables|Default|GetWeapon)) "0, 0, 0" 1.0 1.0 0.0 0 0 0 0)
              (Utilities|FlowControl|Delay 3.72)
              (Variables|Default|SetBulletsFired 0)
              (goto _label Open))))))))

(event EventBeginPlay
  (Utilities|FlowControl|Delay 0.5)
  (CallFunction|MovetoPlace))

(event EventKill/Destroy
  (params (HitImpulse :type Vector :default "0, 0, 0"))
  (bind _mesh (Variables|Character|GetMesh))
  (CallFunction|StopShooting)
  (Variables|/Script/Engine.PrimitiveComponent|SetbGenerateOverlapEvents (Variables|Default|GetBox) false)
  (Collision|SetCollisionEnabled (Variables|Collision|GetCapsuleComponent) "NoCollision")
  (Physics|SetSimulatePhysics _mesh true)
  (Physics|SetPhysicsLinearVelocity _mesh HitImpulse false "None")
  (Utilities|FlowControl|Delay 3.0)
  (Effects|SpawnEmitteratLocation "/Game/DinosRevengeContent/Particles/Blood/P_Blood.P_Blood" (Transformation|GetWorldLocation (Variables|Character|GetMesh)) "0, 0, 0" "2.000000,2.000000,2.000000")
  (Actor|DestroyActor)
  (bind _asbp_dino_gamestate (Utilities|Casting|CastToBP_DinoGamestate (Game|GetGameState)))
  (Default|CheckVictoryCondition _asbp_dino_gamestate))

(fn ConstructionScript
  (CallFunction|SetStartValues (Variables|Default|GetbHeavy)))

(fn GetLeftHandSocket
  (bind _weapon (Variables|Default|GetWeapon))
  (Utilities|IsValid _weapon
    (:Is%20Valid
      (return (Transformation|GetSocketLocation _weapon "LeftHandSocket")))))

(fn TraceandTryHit
  (bind _weapon (Variables|Default|GetWeapon))
  (bind _returnvalue (Transformation|GetWorldRotation _weapon))
  (bind _returnvalue_2 (Transformation|GetWorldLocation _weapon))
  (bind (_outhit _returnvalue_3) (Collision|LineTraceByChannel _returnvalue_2 (+ _returnvalue_2 (* (Math|Vector|GetForwardVector (Math|Rotator|MakeRotator (.roll _returnvalue) (+ (.pitch _returnvalue) (Math|Random|RandomFloatinRange -1e+01 1e+01)) (+ (.yaw _returnvalue) (Math|Random|RandomFloatinRange -2e+01 2e+01)))) -5e+03)) "TraceTypeQuery1" false 0 "ForDuration" true "(R=1.000000,G=0.000000,B=0.000000,A=1.000000)" "(R=0.000000,G=1.000000,B=0.000000,A=1.000000)" 0.5))
  (bind _asbp_dino (Utilities|Casting|CastToBP_Dino (.HitActor (Collision|BreakHitResult _outhit)))
    (:then
      (Default|GetDamage _asbp_dino (Variables|Default|GetDamage))
      (return false))
    (:CastFailed
      (return _returnvalue_3))))

(fn SetStartValues
  (params (bHeavy :type Boolean))
  (Variables|Default|SetShootingTime (Math|Float|SelectFloat 0.1 (Math|Random|RandomFloatinRange 0.25 0.4) bHeavy))
  (Class|SkinnedMeshComponent|SetSkeletalMesh (Variables|Character|GetMesh) (select bHeavy "/Game/DinosRevengeContent/Characters/Humans/HeavySoldier/HeavySoldier.HeavySoldier" "/Game/DinosRevengeContent/Characters/Humans/Soldier/Soldier.Soldier") true))